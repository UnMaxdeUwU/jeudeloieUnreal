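; BP_tuile is a tile that applies a movement effect to the player: advance, go back or teleport, depending on its Mode.
; BeginPlay caches the BP_Player actor, then ApplyColor creates a dynamic material on the Plane to tint it by mode.
; ApllyEffect calls MovePlayer with that mode's value and prints the effect name.
; The tint is noted as broken, and its vector parameter name is None.
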(event `self.ReceiveBeginPlay`
  ; Ref du player
  (bind _returnvalue (`GameplayStatics.GetActorOfClass` "/Game/Project/Blueprinth/BP_Player.BP_Player_C"))
  (set `self.PlayerRef` _returnvalue)
  (`self.ApplyColor`))

(event `ApllyEffect`
  ; Applique l'effet suivant le mode sélectionner
  (switch `int` (`self.Mode`)
    (:`0`
      (`/Game/Project/Blueprinth/BP_Player.MovePlayer` (`self.PlayerRef`) (`self.AdvencedPlayer`))
      (`KismetSystemLibrary.PrintString` "Advenced"))
    (:`1`
      (`/Game/Project/Blueprinth/BP_Player.MovePlayer` (`self.PlayerRef`) (`self.BackPlayer`))
      (`KismetSystemLibrary.PrintString` "Back"))
    (:`2`
      (`/Game/Project/Blueprinth/BP_Player.MovePlayer` (`self.PlayerRef`) (`self.TeleportCase`))
      (`KismetSystemLibrary.PrintString` "Teleport"))))

(event `ApplyColor`
  (bind _plane (`self.Plane`))
  ; Change la couleur mais ne marche pas donc...
  (switch `int` (`self.Mode`)
    (:`0`
      (bind _returnvalue (`PrimitiveComponent.CreateDynamicMaterialInstance` _plane 0 null "None"))
      (`MaterialInstanceDynamic.SetVectorParameterValue` _returnvalue "None" (struct :`G` 1.0 :`A` 1.0)))
    (:`1`
      (bind _returnvalue_2 (`PrimitiveComponent.CreateDynamicMaterialInstance` _plane 0 null "None"))
      (`MaterialInstanceDynamic.SetVectorParameterValue` _returnvalue_2 "None" (struct :`R` 1.0 :`G` 0.876713 :`A` 1.0)))
    (:`2`
      (bind _returnvalue_3 (`PrimitiveComponent.CreateDynamicMaterialInstance` _plane 0 null "None"))
      (`MaterialInstanceDynamic.SetVectorParameterValue` _returnvalue_3 "None" (struct :`R` 1.0 :`A` 1.0)))))

(fn `UserConstructionScript`)