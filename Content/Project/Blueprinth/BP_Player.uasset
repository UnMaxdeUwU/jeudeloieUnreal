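; Board-game player pawn that rolls BP_Dice on the B key and moves along BP_Board's tiles.
; MovePlayer clamps the target index, then StartStep replays a Timeline one tile at a time, forward or backward, lerping actor location.
; At the end it applies a BP_tuile effect (read at current index minus one), or Finish reports the position to the GI game instance.
; Older movement tests remain alongside, partly unwired.
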(event `self.ReceiveBeginPlay`
  ; Initialisation, on récupère la board en ref, le dés et la game instance
  (bind _returnvalue (`GameplayStatics.GetActorOfClass` "/Game/Project/Blueprinth/BP_Board.BP_Board_C"))
  (set `self.Board` _returnvalue)
  (set `self.actuel_pos` 0)
  (bind _returnvalue_2 (`GameplayStatics.GetActorOfClass` "/Game/Project/Blueprinth/BP_Dice.BP_Dice_C"))
  (set `self.Dice` _returnvalue_2)
  (bind _asgi (cast `/Game/Project/GI` (`GameplayStatics.GetGameInstance`)))
  (set `self.As GI` _asgi))

(event `Key|B`
  (params (Key :type "Key Structure"))
  ; Input
  (:`Pressed`
    (`self.PlayDice`)))

(event `PlayFromStart`
  ; Test a oublier, j'ai juste trop mal au coeur de le sup
  (bind (_direction _newtrack_0) (`Timeline|Advanced` :!via `PlayFromStart` :!label _label)
    (:`Update`
      ;; Comment
      (`self.K2_SetActorLocation` (`KismetMathLibrary.VLerp` (`self.K2_GetActorLocation`) (`self.K2_GetActorLocation` (`|GetArrayItem` (`/Game/Project/Blueprinth/BP_Board.Tuile` (`self.Board`)) (+ (`self.I`) (`self.actuel_pos`)))) _newtrack_0) true))
    (:`Finished`
      (bind _result (`/Engine/EditorBlueprintResources/StandardMacros.IncrementInt` (`self.I`))
        (:`  `
          (if (>= _result 0)
            (set `self.actuel_pos` (`self.Desiredposition`) :!label _label_2)
            (set `self.I` 0)
            (bind _asbp_tuile (cast `/Game/Project/Blueprinth/BP_tuile` (`|GetArrayItem` (`/Game/Project/Blueprinth/BP_Board.Tuile` (`self.Board`)) (`self.Desiredposition`)))
              (:`then`
                (`self.New time`)
                (`self.PlayFromStart`)
                (`/Game/Project/Blueprinth/BP_tuile.ApllyEffect` _asbp_tuile))
              (:`CastFailed`
                (`self.Finish`)))
            (else
              (`self.New time` :!label _label_3)
              (`self.PlayFromStart`)
              (`self.FromStart`)
              (`self.New Timee`))))))))

(event `/Game/Project/BPI/DiceValue.DiceValue`
  (params (NewParam1 :type Integer))
  ; On obtient la valeur du dés qui vient d'être lancer
  (bind _output_get (set `self.valueofDice` NewParam1))
  (`KismetSystemLibrary.PrintString` (`KismetStringLibrary.Conv_IntToString` _output_get)))

(event `New time`
  ; Test a oublier, j'ai juste trop mal au coeur de le sup
  (goto _label :!via `SetNewTime`))

(event `FromStart`
  ; Test a oublier, j'ai juste trop mal au coeur de le sup
  (`Timeline|Back` :!via `PlayFromStart` :!label _label_4
    (:`Update`
      (`self.K2_SetActorLocation` (`KismetMathLibrary.VLerp` (`self.K2_GetActorLocation`) (`self.K2_GetActorLocation` (`|GetArrayItem` (`/Game/Project/Blueprinth/BP_Board.Tuile` (`self.Board`)) (- (`self.I`) (`self.actuel_pos`))))) true))
    (:`Finished`
      (bind _result (`/Engine/EditorBlueprintResources/StandardMacros.DecrementInt` (`self.I`))
        (:`  `
          (if (<= _result 0)
            (goto _label_2)
            (else
              (goto _label_3))))))))

(event `PlayDice`
  ; On lance le dés on on envoie la valeur de déplacement
  (`/Game/Project/Blueprinth/BP_Dice.BeginDice` (`self.Dice`))
  (`self.MovePlayer` (`self.valueofDice`)))

(event `New Timee`
  ; Test a oublier, j'ai juste trop mal au coeur de le sup
  (goto _label_4 :!via `SetNewTime`))

(event `MovePlayer`
  (params (Mouvement :type Integer))
  ; On vérifie si ma position actuel est égale à la position rechercher
  (bind _output_get (set `self.Desiredposition` (`KismetMathLibrary.Clamp` (+ (`self.Desiredposition`) Mouvement) 0 (- (`KismetArrayLibrary.Array_Length` (`/Game/Project/Blueprinth/BP_Board.Tuile` (`self.Board`))) 1))))
  (if (not (== _output_get (`self.actuel_pos`)))
    ; On commence le déplacement de 1 case par 1 case
    (set `self.IsMoving` true)
    (`self.StartStep`)))

(event `StartStep`
  (if (== (`self.Desiredposition`) (`self.actuel_pos`))
    (set `self.IsMoving` false)
    ; Quand on a finit tout les déplacements, si la tuile sur laquelle on a atterit est un actor tuile alors on applique l'effet.
    (bind _asbp_tuile (cast `/Game/Project/Blueprinth/BP_tuile` (`|GetArrayItem` (`/Game/Project/Blueprinth/BP_Board.Tuile` (`self.Board`)) (- (`self.actuel_pos`) 1)))
      (:`then`
        (`/Game/Project/Blueprinth/BP_tuile.ApllyEffect` _asbp_tuile))
      (:`CastFailed`
        (`self.Finish`)))
    (else
      (`KismetSystemLibrary.PrintString` "Start moving")
      ; On vérifie si le nombre est positif ou négatif, si le nombre est négatif alors direction = -1 si le nombre est positif alors direction = 1
      (set `self.Direction` (`KismetMathLibrary.SignOfInteger` (- (`self.Desiredposition`) (`self.actuel_pos`))))
      (set `self.StartPos` (`self.K2_GetActorLocation`))
      (set `self.EndPos` (`self.K2_GetActorLocation` (`|GetArrayItem` (`/Game/Project/Blueprinth/BP_Board.Tuile` (`self.Board`)) (+ (`self.actuel_pos`) (`self.Direction`)))))
      (bind (_direction _newtrack_0) (`Timeline|Timeline` :!via `PlayFromStart`)
        (:`Update`
          (`self.K2_SetActorLocation` (`KismetMathLibrary.VLerp` (`self.K2_GetActorLocation`) (`self.K2_GetActorLocation` (`|GetArrayItem` (`/Game/Project/Blueprinth/BP_Board.Tuile` (`self.Board`)) (+ (`self.I`) (`self.actuel_pos`)))) _newtrack_0) true))
        (:`Finished`
          ; On ajoute un fois le déplacement finit notre position actuel
          (bind _output_get (set `self.actuel_pos` (+ (`self.actuel_pos`) (`self.Direction`))))
          (`KismetSystemLibrary.PrintString` (`KismetStringLibrary.Conv_IntToString` _output_get))
          ; On recommence
          (`self.StartStep`))))))

(fn `Finish`
  (`KismetSystemLibrary.PrintString` "Fin")
  (`/Game/Project/GI.PlayerPosition` (`self.As GI`) (`self.Desiredposition`)))

(fn `UserConstructionScript`)